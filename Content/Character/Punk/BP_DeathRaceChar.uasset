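; BP_DeathRaceChar is a player character for a death race mode that moves along the world X axis at walk or run pace.
; On BeginPlay it adds the IMC_DeathRace Enhanced Input mapping context to its player controller.
; IA_MoveFast toggles a running flag, which selects the X magnitude of the direction IA_Move passes to AddMovementInput, so speed changes through input strength alone.
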(event `self.ReceiveBeginPlay`
  (bind _asplayer_controller (cast `PlayerController` (`self.GetController`)))
  (message `EnhancedInputSubsystemInterface.AddMappingContext` (pcsubsystem `EnhancedInputLocalPlayerSubsystem` _asplayer_controller) "/Game/Character/Input/IMC_DeathRace.IMC_DeathRace" 0 (struct)))

(event `EnhancedInput|/Game/Character/Input/IA_Move`
  (params (ActionValue :type "Vector2D Structure") (ElapsedSeconds :type "Float (double-precision)") (TriggeredSeconds :type "Float (double-precision)") (InputAction :type "InputAction Object Reference" :default "/Game/Character/Input/IA_Move.IA_Move"))
  (:`Triggered`
    (`self.AddMovementInput` (`KismetMathLibrary.MakeVector` (`KismetMathLibrary.SelectFloat` 0.8 0.4 (`self.IsRunning`))) ActionValue_X)))

(event `EnhancedInput|/Game/Character/Input/IA_MoveFast`
  (params (ActionValue :type Boolean) (ElapsedSeconds :type "Float (double-precision)") (TriggeredSeconds :type "Float (double-precision)") (InputAction :type "InputAction Object Reference" :default "/Game/Character/Input/IA_MoveFast.IA_MoveFast"))
  (:`Triggered`
    (set `self.IsRunning` true))
  (:`Completed`
    (set `self.IsRunning` false)))

(fn `UserConstructionScript`)