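; BP_DeathRaceChar_NPC is a Death Race NPC character that alternates at random between standing idle and walking.
; A self-rearming timer with a random delay fires RandomMove, which flips IsIdle.
; While not idle, Tick feeds constant movement input along world X.
; Once DidReceiveHit is set, Tick stops that input and clears the timer a single time through a DoOnce.
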(event `self.ReceiveBeginPlay`
  (bind _output_get (set `self.timerDelay` (`KismetMathLibrary.RandomFloatInRange` 0.1 7.0) :!label _label))
  (bind _returnvalue (`KismetSystemLibrary.K2_SetTimerDelegate` (delegate `RandomMove`) _output_get)))

(event `self.ReceiveTick`
  (params (DeltaSeconds :type "Float (single-precision)"))
  (if (`self.DidReceiveHit`)
    (`/Engine/EditorBlueprintResources/StandardMacros.DoOnce` false
      (:`Completed`
        (`KismetSystemLibrary.K2_ClearAndInvalidateTimerHandle` (stale `self.ReceiveBeginPlay` _returnvalue))))
    (elif (not (`self.IsIdle`))
      (`self.AddMovementInput` (0.4 0.0 0.0)))))

(event `RandomMove`
  (if (`self.IsIdle`)
    (set `self.IsIdle` false)
    (goto _label)
    (else
      (set `self.IsIdle` true)
      (goto _label))))

(fn `UserConstructionScript`)