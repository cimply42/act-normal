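; BP_Civilian_Imposter is the player-controlled imposter civilian in what appears to be a Five Statues game, printing "game over" once five statues are touched.
; Enhanced Input drives movement and records facing direction, while Space or a gamepad button sets an attack-held flag.
; IsStuck flags held movement with low velocity, and Hit sphere-traces along the last input direction to mark an NPC civilian as hit; neither is called here.
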(event `self.ReceiveBeginPlay`
  (bind _asplayer_controller (cast `PlayerController` (`self.GetController`)))
  (`EnhancedInputSubsystemInterface.AddMappingContext` (pcsubsystem `EnhancedInputLocalPlayerSubsystem` _asplayer_controller) "/Game/Character/Input/IMC_FiveStatues.IMC_FiveStatues" 0 (struct)))

(event `self.ReceiveTick`
  (params (DeltaSeconds :type "Float (single-precision)"))
  (if (>= (`self.NumStatuesTouched`) 5)
    (`/Engine/EditorBlueprintResources/StandardMacros.DoOnce` false
      (:`Completed`
        (`KismetSystemLibrary.PrintString` "game over")))))

(event `EnhancedInput|/Game/Character/Input/IA_Move`
  (params (ActionValue :type "Vector2D Structure") (ElapsedSeconds :type "Float (double-precision)") (TriggeredSeconds :type "Float (double-precision)") (InputAction :type "InputAction Object Reference" :default "/Game/Character/Input/IA_Move.IA_Move"))
  (:`Triggered`
    (`self.AddMovementInput` (0.5 0.0 0.0) ActionValue_X) ; left/right
    (`self.AddMovementInput` (0.0 -0.5 0.0) ActionValue_Y) ; up/down
    (set `self.Directionality` (`KismetMathLibrary.MakeVector2D` ActionValue_X ActionValue_Y)))
  (:`Started`
    (set `self.IsHoldingMove` true))
  (:`Completed`
    (set `self.IsHoldingMove` false)))

(event `Key|SpaceBar`
  (params (Key :type "Key Structure"))
  (:`Pressed`
    (set `self.IsHoldingAttack` true :!label _label))
  (:`Released`
    (set `self.IsHoldingAttack` false :!label _label_2)))

(event `Key|Gamepad_Special_Right`
  (params (Key :type "Key Structure"))
  (:`Pressed`
    (goto _label))
  (:`Released`
    (goto _label_2)))

(fn `Hit`
  (bind _returnvalue (`self.K2_GetActorLocation`))
  (bind _outhit (`KismetSystemLibrary.SphereTraceSingleForObjects` :`Start` _returnvalue :`End` (+ _returnvalue (* (`self.Directionality`) (70.0 -70.0))) :`Radius` 10.0 :`ObjectTypes` (`|MakeArray` "ObjectTypeQuery3" :!type "EObjectTypeQuery Enum") :`DrawDebugType` "ForDuration"))
  (bind _asbp_civilian_npc (cast `/Game/Character/BP_Civilian_NPC` (`.HitActor` (`GameplayStatics.BreakHitResult` _outhit))))
  (set `/Game/Character/BP_Civilian_NPC.DidReceiveHit` true _asbp_civilian_npc))

(fn `IsStuck`
  (returns (IsStuck :type Boolean))
  (return (and (< (`KismetMathLibrary.VSize` (`self.GetVelocity`)) (`self.StuckThreshold`)) (`self.IsHoldingMove`))))

(fn `UserConstructionScript`)