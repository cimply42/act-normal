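; BP_Civilian is a player-controlled civilian character with Enhanced Input movement and an attack.
; Move input drives look and fixed world-axis movement, passing its direction through an RPC-named event into Directionality.
; Attack input or gamepad Special Right toggles IsHoldingAttack through similar events.
; HitDetect, not called here, sphere-traces pawns at the right foot and flags struck BP_Civilian or BP_Civilian_NPC_2 actors with DidReceiveHit.
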(event `self.ReceiveBeginPlay`
  (bind _asplayer_controller (cast `PlayerController` (`self.GetController`)))
  (`EnhancedInputSubsystemInterface.AddMappingContext` (pcsubsystem `EnhancedInputLocalPlayerSubsystem` _asplayer_controller) "/Game/Character/Input/IMC_FiveStatues.IMC_FiveStatues" 0 (struct)))

(event `EnhancedInput|/Game/Character/Input/IA_Move`
  (params (ActionValue :type "Vector2D Structure") (ElapsedSeconds :type "Float (double-precision)") (TriggeredSeconds :type "Float (double-precision)") (InputAction :type "InputAction Object Reference" :default "/Game/Character/Input/IA_Move.IA_Move"))
  (:`Triggered`
    (`self.AddControllerYawInput` ActionValue_X) ; look left/right
    (`self.AddControllerPitchInput` ActionValue_Y) ; look up/down
    (`self.AddMovementInput` (0.5 0.0 0.0) ActionValue_X) ; left/right
    (`self.AddMovementInput` (0.0 -0.5 0.0) ActionValue_Y) ; up/down
    (bind _output_get (set `self.Directionality` (`KismetMathLibrary.MakeVector2D` ActionValue_X ActionValue_Y)))
    (`self.RPC_SetServerDirectionality` _output_get)))

(event `RPC_SetServerDirectionality`
  (params (Directionality :type "Vector2D Structure"))
  (set `self.Directionality` Directionality))

(event `EnhancedInput|/Game/Character/Input/IA_Attack`
  (params (ActionValue :type Boolean) (ElapsedSeconds :type "Float (double-precision)") (TriggeredSeconds :type "Float (double-precision)") (InputAction :type "InputAction Object Reference" :default "/Game/Character/Input/IA_Attack.IA_Attack"))
  (:`Triggered`
    (`KismetSystemLibrary.PrintString` "attack")
    (`self.RPC_HitStart` :!label _label))
  (:`Completed`
    (`self.RPC_HitComplete` :!label _label_2)))

(event `Key|Gamepad_Special_Right`
  (params (Key :type "Key Structure"))
  (:`Pressed`
    (goto _label))
  (:`Released`
    (goto _label_2)))

(event `RPC_HitStart`
  (set `self.IsHoldingAttack` true))

(event `RPC_HitComplete`
  (set `self.IsHoldingAttack` false))

(event `RPC_AttackCompleted`)

(fn `HitDetect`
  (bind _returnvalue (`SceneComponent.GetSocketLocation` (`self.Mesh`) "Foot_R"))
  (bind _outhit (`KismetSystemLibrary.SphereTraceSingleForObjects` :`Start` _returnvalue :`End` _returnvalue :`Radius` 50.0 :`ObjectTypes` (`|MakeArray` "ObjectTypeQuery3" :!type "EObjectTypeQuery Enum") :`DrawDebugType` "ForDuration"))
  (bind (_bblockinghit _binitialoverlap _time _distance _location _impactpoint _normal _impactnormal _physmat _hitactor) (`GameplayStatics.BreakHitResult` _outhit))
  (bind _asbp_civilian (cast `/Game/Character/BP_Civilian` _hitactor)
    (:`then`
      (set `/Game/Character/BP_Civilian.DidReceiveHit` true _asbp_civilian))
    (:`CastFailed`
      (bind _asbp_civilian_npc_2 (cast `/Game/Character/BP_Civilian_NPC_2` _hitactor))
      (set `/Game/Character/BP_Civilian_NPC_2.DidReceiveHit` true _asbp_civilian_npc_2))))

(fn `RPC_AttackStarted`)

(fn `RPC_MoveCompleted`)

(fn `RPC_MoveStarted`)

(fn `UserConstructionScript`)