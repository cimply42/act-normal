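; BP_Civilian_NPC is a civilian character that wanders randomly until it receives a hit.
; A randomly delayed timer re-arms itself through RandomMove, alternating between idling and picking a new direction from a set of movement values.
; Tick feeds that direction into movement input while the civilian is not idle.
; Once a hit is received, Tick stops applying movement and clears the timer once.
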(event `self.ReceiveBeginPlay`
  (bind _output_get (set `self.timerDelay` (`KismetMathLibrary.RandomFloatInRange` 0.5 7.0) :!label _label))
  (bind _returnvalue (`KismetSystemLibrary.K2_SetTimerDelegate` (delegate `RandomMove`) _output_get)))

(event `RandomMove`
  (bind _movedirectionvalues (`self.MoveDirectionValues`))
  (bind _isidleorstationary (`self.IsIdleOrStationary`))
  (if _isidleorstationary
    (set `self.IsIdle` false)
    (bind _output_get (set `self.Directionality` (`KismetMathLibrary.MakeVector2D` (`KismetArrayLibrary.Array_Random` _movedirectionvalues) (`KismetArrayLibrary.Array_Random` _movedirectionvalues))))
    (bind _result (`/Engine/EditorBlueprintResources/StandardMacros.NegateFloat` (`.Y` (`KismetMathLibrary.BreakVector2D` _output_get)))
      (:`  `
        (goto _label)))
    (else
      (set `self.IsIdle` true)
      (goto _label))))

(event `self.ReceiveTick`
  (params (DeltaSeconds :type "Float (single-precision)"))
  (if (`self.DidReceiveHit`)
    (`/Engine/EditorBlueprintResources/StandardMacros.DoOnce` false
      (:`Completed`
        (`KismetSystemLibrary.K2_ClearAndInvalidateTimerHandle` (stale `self.ReceiveBeginPlay` _returnvalue))))
    (elif (not (`self.IsIdle`))
      (`self.AddMovementInput` (`KismetMathLibrary.MakeVector` (`KismetMathLibrary.BreakVector2D` (stale `RandomMove` _output_get)) (stale `RandomMove` _result))))))

(fn `IsIdleOrStationary`
  (returns (IsIdleOrStationary :type Boolean))
  (return (or (`self.IsIdle`) (`KismetMathLibrary.EqualExactly_Vector2DVector2D` (`self.Directionality`)))))

(fn `UserConstructionScript`)